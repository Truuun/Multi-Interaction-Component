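; BP_BlockSolutionChecker watches a set of changing blocks and reveals a particle effect when they match a configured solution.
; On BeginPlay it hides the particles and binds to each block's change event.
; Each change compares every block's shrunk state and first cube material against the expected values in the Blocks array.
; A full match shows the particles, which are never hidden again afterward.
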(event `self.ReceiveBeginPlay`
  (`SceneComponent.SetVisibility` (`self.ParticleSystem`) false false)
  ;[1 1 1] "Listen" to the change event of each block that is part of this solution
  (for _array_element (`self.Blocks`)
    (add `/Game/InteractionExamples/InteractionObjects/ChangingBlock/BP_ChangingBlock.OnBlockChange` (`.Block_6_7DC248984BF879864855D1B71F316369` (break `/Game/InteractionExamples/InteractionObjects/ChangingBlock/FBlockConfiguration` _array_element)) (delegate `OnCheckSolution`))))

(event `OnCheckSolution`
  (bind _issolution (`self.IsSolution`))
  (if _issolution
    (`SceneComponent.SetVisibility` (`self.ParticleSystem`) true false)))

(fn `IsSolution`
  (returns (IsSolution :type Boolean))
  ;[1 1 1] Go through each block and check if its configuration matches
  (for _array_element (`self.Blocks`)
    (bind (_block _isshrunk _material) (break `/Game/InteractionExamples/InteractionObjects/ChangingBlock/FBlockConfiguration` _array_element))
    (if (!= (`/Game/InteractionExamples/InteractionObjects/ChangingBlock/BP_ChangingBlock.bIsShrunk` _block) _isshrunk)
      (return false)
      (elif (!= _material (`|GetArrayItem` (`MeshComponent.GetMaterials` (`/Game/InteractionExamples/InteractionObjects/ChangingBlock/BP_ChangingBlock.Cube` _block))))
        (return false))))
  (return true))

(fn `UserConstructionScript`)