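; Example interactable block whose size and color the player changes through a MultiInteraction component.
; On BeginPlay it registers a shrink/reset action and one action per selectable color, mapping each action handle to its material.
; Resizing toggles actor scale and renames its action, while choosing a color swaps the cube material and disables that color's action.
; Both changes fire the OnBlockChange dispatcher, which a solution checker uses to track the cubes.
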(event `self.ReceiveBeginPlay`
  (`|ExecutionSequence`
    (:`then_0`
      ;[1 1 1] Add action for shrinking and resetting size, in this case we simply update the action text after the shrinking or resetting is done
      (bind _returnvalue (`MultiInteractionComponent.AddAction_Fixed` (`self.MultiInteraction`) (delegate `Resize`) "Shrink" "ENABLED")) ; In this case we set the action's text when the objects size is changed
      (`self.UpdateSize` _returnvalue))
    (:`then_1`
      ;[1 1 1] Add an interation for each material that can be selected and set the starting color
      (for (_array_element _array_index) (`self.SelectableColors`)
        (bind (_actionnname _material) (break `/Game/InteractionExamples/InteractionObjects/ChangingBlock/FSelectableColors` _array_element))
        (bind _returnvalue_2 (`MultiInteractionComponent.AddAction_Fixed` (`self.MultiInteraction`) (delegate `OnColorChange`) _actionnname "ENABLED")) ; In this case, we set the visibility manually when a new color is selected
        (`BlueprintMapLibrary.Map_Add` (`self.HandleToMaterialMap`) _returnvalue_2 _material)
        (if (== _array_index (`self.StartingColor`))
          (`MultiInteractionComponent.SetActionVisibility` (`self.MultiInteraction`) _returnvalue_2 "DISABLED")
          (`PrimitiveComponent.SetMaterial` (`self.Cube`) 0 _material)
          (set `self.LastChoice` _returnvalue_2))))))

(event `Resize`
  (params (Handle :type "InterativeActionHandle Structure") (User :type "Actor Object Reference"))
  ;[1 1 1] Add action for shrinking and resetting size, in this case we simply update the action text after the shrinking or resetting is done
  (set `self.bIsShrunk` (not (`self.bIsShrunk`)))
  (`self.UpdateSize` Handle)
  (`self.OnBlockChange`) ; This dispatcher is used by the solution checker to track changes in the cubes
)

(event `OnColorChange`
  (params (Handle :type "InterativeActionHandle Structure") (User :type "Actor Object Reference"))
  ;[1 1 1] Sets the material of the cube based on chosen action handle and disable that handle as it is currently that color
  (`PrimitiveComponent.SetMaterial` (`self.Cube`) 0 (`BlueprintMapLibrary.Map_Find` (`self.HandleToMaterialMap`) Handle))
  (`MultiInteractionComponent.SetActionVisibility` (`self.MultiInteraction`) (`self.LastChoice`) "ENABLED")
  (`MultiInteractionComponent.SetActionVisibility` (`self.MultiInteraction`) Handle "DISABLED")
  (set `self.LastChoice` Handle)
  (`self.OnBlockChange`) ; This dispatcher is used by the solution checker to track changes in the cubes
)

(fn `UpdateSize`
  (params (NewParam :type "InterativeActionHandle Structure"))
  (if (`self.bIsShrunk`)
    (`self.SetActorScale3D` (0.5 0.5 0.5))
    (`MultiInteractionComponent.SetActionName` (`self.MultiInteraction`) NewParam "Reset")
    (else
      (`self.SetActorScale3D` (1.0 1.0 1.0))
      (`MultiInteractionComponent.SetActionName` (`self.MultiInteraction`) NewParam "Shrink"))))

(fn `UserConstructionScript`)