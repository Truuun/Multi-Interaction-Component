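; Example interaction statue that collects berries from the player and opens a sliding wall once the required count is reached.
; On BeginPlay it registers an "Add Berry" action on its MultiInteraction component, with bindings for the action, its label and its visibility.
; Adding a berry takes one from the interaction character and updates the displayed collected/required name.
; The action is disabled when the player has no berries and hidden once complete.
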(event `self.ReceiveBeginPlay`
  (`MultiInteractionComponent.AddAction` (`self.MultiInteraction`) (delegate `OnAddBerry`) (`|CreateDelegate` :!event `GetActionName`) (`|CreateDelegate` :!event `GetActionVisibility`))
  (`self.UpdateObjectName`))

(event `OnAddBerry`
  (params (Handle :type "InterativeActionHandle Structure") (User :type "Actor Object Reference"))
  ;[1 1 1] Removes a berry from the player, adding it to this object and check if it is enough to open the door
  (bind _asbp_interaction_character (cast `/Game/InteractionExamples/Character/BP_InteractionCharacter` User))
  (`/Game/InteractionExamples/Character/BP_InteractionCharacter.RemoveBerry` _asbp_interaction_character)
  (`/Engine/EditorBlueprintResources/StandardMacros.IncrementInt` (`self.CurrentBerriesCount`)
    (:`  `
      (`self.UpdateObjectName`)
      (if (== (`self.RequiredBerriesCount`) (`self.CurrentBerriesCount`))
        (`/Game/InteractionExamples/InteractionObjects/BP_SlidingWall.OnSlideOpen` (`self.SlidingWall`))))))

(fn `GetActionName`
  (params (Handle :type "InterativeActionHandle Structure") (User :type "Actor Object Reference"))
  (returns (Name :type Text))
  (bind _asbp_interaction_character (cast `/Game/InteractionExamples/Character/BP_InteractionCharacter` User))
  (return (`KismetTextLibrary.Conv_StringToText` (`KismetStringLibrary.BuildString_Int` "Add Berry: " "" (`/Game/InteractionExamples/Character/BP_InteractionCharacter.GetBerriesCount` _asbp_interaction_character) " left"))))

(fn `GetActionVisibility`
  (params (Handle :type "InterativeActionHandle Structure") (User :type "Actor Object Reference"))
  (returns (NewParam2 :type "EInteractionVisibility Enum"))
  (if (== (`self.CurrentBerriesCount`) (`self.RequiredBerriesCount`))
    (return "HIDDEN")
    (else
      (bind _asbp_interaction_character (cast `/Game/InteractionExamples/Character/BP_InteractionCharacter` User))
      (if (> (`/Game/InteractionExamples/Character/BP_InteractionCharacter.GetBerriesCount` _asbp_interaction_character) 0)
        (return "ENABLED")
        (else
          (return "DISABLED"))))))

(fn `UpdateObjectName`
  (`MultiInteractionComponent.SetInteractionName` (`self.MultiInteraction`) (`KismetTextLibrary.Conv_StringToText` (`KismetStringLibrary.Concat_StrStr` "Berry Collector " "(" (`KismetStringLibrary.Conv_IntToString` (`self.CurrentBerriesCount`)) "/" (`KismetStringLibrary.Conv_IntToString` (`self.RequiredBerriesCount`)) ")"))))

(fn `UserConstructionScript`)