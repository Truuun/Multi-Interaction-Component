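; Example interactable door that users can open, close, lock and unlock through a MultiInteraction component.
; BeginPlay snaps the mesh to match DoorState and registers both actions, whose names update with the state.
; A timeline swings the mesh's yaw, playing forward to open and backward to close.
; Visibility callbacks disable Open/Close while locked or moving, and hide Lock/Unlock while open or moving.
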(event `self.ReceiveBeginPlay`
  (`|ExecutionSequence`
    (:`then_0`
      (bind _returnvalue (`MultiInteractionComponent.AddAction_FixedName` (`self.MultiInteraction`) (delegate `OnOpenDoor`) "Open Door" (`|CreateDelegate` :!event `GetOpenActionVisibility`))) ; In this case, the name of the action is set when the door is opened or closed
      ;[1 1 1] Make sure the door starts in the correct state physically
      (switch `/Game/InteractionExamples/InteractionObjects/Door/EDoorState` (`self.DoorState`)
        (:`NewEnumerator0`
          (`SceneComponent.K2_SetRelativeRotation` (`self.StaticMesh`) (struct :`Yaw` 90.0) false false)
          (`MultiInteractionComponent.SetActionName` (`self.MultiInteraction`) _returnvalue "Close"))
        (:`NewEnumerator1`
          (`SceneComponent.K2_SetRelativeRotation` :`self` (`self.StaticMesh`) :!label _label)
          (`MultiInteractionComponent.SetActionName` (`self.MultiInteraction`) _returnvalue "Open"))
        (:`NewEnumerator2`
          (goto _label))))
    (:`then_1`
      ;[1 1 1] Add an action for locking the door
      (bind _returnvalue_2 (`MultiInteractionComponent.AddAction_FixedName` (`self.MultiInteraction`) (delegate `OnLock`) "Lock Door" (`|CreateDelegate` :!event `GetLockActionVisibility`))) ; In this case, we set the name of the action when the door is locked or unlocked
      (set `self.LockActionHandle` _returnvalue_2)
      (`self.UpdateLockState`))))

(event `OnOpenDoor`
  (params (Handle :type "InterativeActionHandle Structure") (User :type "Actor Object Reference"))
  ;[1 1 1] Open or close the door
  (switch `/Game/InteractionExamples/InteractionObjects/Door/EDoorState` (`self.DoorState`)
    (:`NewEnumerator0`
      (set `self.DoorState` "NewEnumerator1")
      (set `self.bIsChangingState` true)
      (`MultiInteractionComponent.SetActionName` (`self.MultiInteraction`) Handle "Open Door")
      (bind (_direction _newtrack_0) (`Timeline|DoorTransition` :!via `ReverseFromEnd` :!label _label_2)
        (:`Update`
          (`SceneComponent.K2_SetRelativeRotation` (`self.StaticMesh`) (`KismetMathLibrary.MakeRotator` 0.0 0.0 _newtrack_0) false false))
        (:`Finished`
          (set `self.bIsChangingState` false))))
    (:`NewEnumerator1`
      (set `self.DoorState` "NewEnumerator0")
      (set `self.bIsChangingState` true)
      (`MultiInteractionComponent.SetActionName` (`self.MultiInteraction`) Handle "Close Door")
      (goto _label_2 :!via `PlayFromStart`))))

(event `OnLock`
  (params (Handle :type "InterativeActionHandle Structure") (User :type "Actor Object Reference"))
  ;[1 1 1] Add an action for locking the door
  (switch `/Game/InteractionExamples/InteractionObjects/Door/EDoorState` (`self.DoorState`)
    (:`NewEnumerator1`
      (set `self.DoorState` "NewEnumerator2"))
    (:`NewEnumerator2`
      (set `self.DoorState` "NewEnumerator1")))
  (`self.UpdateLockState`))

(fn `GetLockActionVisibility`
  (params (Handle :type "InterativeActionHandle Structure") (User :type "Actor Object Reference"))
  (returns (NewParam1 :type "EInteractionVisibility Enum"))
  (if (and (not (`self.bIsChangingState`)) (`|EnumInequality` (`self.DoorState`) "NewEnumerator0"))
    (return "ENABLED")
    (else
      (return "HIDDEN"))))

(fn `GetOpenActionVisibility`
  (params (Handle :type "InterativeActionHandle Structure") (User :type "Actor Object Reference"))
  (returns (NewParam1 :type "EInteractionVisibility Enum"))
  (if (or (`self.bIsChangingState`) (`|EnumEquality` (`self.DoorState`) "NewEnumerator2"))
    (return "DISABLED")
    (else
      (return "ENABLED"))))

(fn `UpdateLockState`
  (switch `/Game/InteractionExamples/InteractionObjects/Door/EDoorState` (`self.DoorState`)
    (:`NewEnumerator1`
      (`MultiInteractionComponent.SetActionName` (`self.MultiInteraction`) (`self.LockActionHandle`) "Lock Door")
      (`MultiInteractionComponent.SetInteractionName` (`self.MultiInteraction`) "Door"))
    (:`NewEnumerator2`
      (`MultiInteractionComponent.SetActionName` (`self.MultiInteraction`) (`self.LockActionHandle`) "Unlock Door")
      (`MultiInteractionComponent.SetInteractionName` (`self.MultiInteraction`) "Door (Locked)"))))

(fn `UserConstructionScript`)