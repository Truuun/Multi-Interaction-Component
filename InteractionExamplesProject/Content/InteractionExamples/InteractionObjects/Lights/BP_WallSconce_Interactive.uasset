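; Interactive wall sconce example whose light players can switch on and off or brighten and dim in steps.
; BeginPlay registers three fixed actions on the MultiInteraction component; the switch action renames itself to match the light state.
; After each brightness step, CheckBrightnessFunctions disables any action that would leave the allowed range, and intensity is applied only while lit.
; The construction script applies brightness, color and cone angles to the light.
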(event `self.ReceiveBeginPlay`
  (`|ExecutionSequence`
    (:`then_0`
      ;[1 1 1] Turn the light on or off
      (bind _returnvalue (`MultiInteractionComponent.AddAction_Fixed` (`self.MultiInteraction`) (delegate `OnLightSwitch`) "Turn Off" "ENABLED"))
      (`self.UpdateLightState` _returnvalue))
    (:`then_1`
      ;[1 1 1] Increase or decrease the brightness of the light
      (bind _returnvalue_2 (`MultiInteractionComponent.AddAction_Fixed` (`self.MultiInteraction`) (delegate `OnIncreaseBrightness`) "Increase Brigthness" "ENABLED"))
      (set `self.IncreaseHandle` _returnvalue_2))
    (:`then_2`
      (bind _returnvalue_3 (`MultiInteractionComponent.AddAction_Fixed` (`self.MultiInteraction`) (delegate `OnDecreaseBrightness`) "Decrease Brigthness" "ENABLED"))
      (set `self.DecreaseHandle` _returnvalue_3))
    (:`then_3`
      (`self.CheckBrightnessFunctions`))))

(event `OnLightSwitch`
  (params (Handle :type "InterativeActionHandle Structure") (User :type "Actor Object Reference"))
  ;[1 1 1] Turn the light on or off
  (set `self.bIsTurnedOn` (not (`self.bIsTurnedOn`)))
  (`self.UpdateLightState` Handle))

(event `OnIncreaseBrightness`
  (params (Handle :type "InterativeActionHandle Structure") (User :type "Actor Object Reference"))
  ;[1 1 1] Increase or decrease the brightness of the light
  (set `self.CurrentBrightness` (+ (`self.CurrentBrightness`) (`self.BrigthnessStepSize`)))
  (`self.CheckBrightnessFunctions` :!label _label)
  (if (`self.bIsTurnedOn`)
    (`LightComponent.SetIntensity` (`self.PointLight2`) (`self.CurrentBrightness`))))

(event `OnDecreaseBrightness`
  (params (Handle :type "InterativeActionHandle Structure") (User :type "Actor Object Reference"))
  ;[1 1 1] Increase or decrease the brightness of the light
  (set `self.CurrentBrightness` (- (`self.CurrentBrightness`) (`self.BrigthnessStepSize`)))
  (goto _label))

(fn `CheckBrightnessFunctions`
  ;[1 1 1] Don't show the "increase brigthness" action if it would exceed the maximum brightness
  (if (> (+ (`self.CurrentBrightness`) (`self.BrigthnessStepSize`)) (+ (`self.MinBrightness`) (`self.MaxBrightnessIncrease`)))
    (`MultiInteractionComponent.SetActionVisibility` (`self.MultiInteraction`) (`self.IncreaseHandle`) "DISABLED")
    (else
      (`MultiInteractionComponent.SetActionVisibility` (`self.MultiInteraction`) (`self.IncreaseHandle`) "ENABLED")))
  ;[1 1 1] Don't show the "decrease brigthness" action if it would get below the minimum brightness
  (if (< (- (`self.CurrentBrightness`) (`self.BrigthnessStepSize`)) (`self.MinBrightness`))
    (`MultiInteractionComponent.SetActionVisibility` (`self.MultiInteraction`) (`self.DecreaseHandle`) "DISABLED")
    (else
      (`MultiInteractionComponent.SetActionVisibility` (`self.MultiInteraction`) (`self.DecreaseHandle`) "ENABLED"))))

(fn `UpdateLightState`
  (params (Handle :type "InterativeActionHandle Structure"))
  (if (`self.bIsTurnedOn`)
    (`MultiInteractionComponent.SetActionName` (`self.MultiInteraction`) Handle "Turn Off")
    (`LightComponent.SetIntensity` (`self.PointLight2`) (`self.CurrentBrightness`))
    (else
      (`MultiInteractionComponent.SetActionName` (`self.MultiInteraction`) Handle "Turn On")
      (`LightComponent.SetIntensity` (`self.PointLight2`) 0.0))))

(fn `UserConstructionScript`
  (bind _pointlight2 (`self.PointLight2`))
  (`LightComponent.SetIntensity` _pointlight2 (`self.CurrentBrightness`))
  (`LightComponent.SetLightColor` _pointlight2 (`self.Color`) true)
  (`SpotLightComponent.SetInnerConeAngle` _pointlight2 (`self.Inner Cone Angle`))
  (`SpotLightComponent.SetOuterConeAngle` _pointlight2 (`self.Outer Cone Angle`)))