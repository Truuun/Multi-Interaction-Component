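; BP_Bush is an interaction example bush that lets players pick berries, with a cooldown between picks.
; On BeginPlay it registers a pick action on its MultiInteraction component, with bindings for execution, name and visibility.
; Picking starts a timer and adds a berry to the interacting BP_InteractionCharacter.
; During cooldown the action is disabled and its dynamic label shows the seconds remaining.
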(event `self.ReceiveBeginPlay`
  (`MultiInteractionComponent.AddAction` (`self.MultiInteraction`) (delegate `OnPickBerry`) (`|CreateDelegate` :!event `GetActionPickName`) (`|CreateDelegate` :!event `GetActionPickVisibility`)))

(event `OnPickBerry`
  (params (Handle :type "InterativeActionHandle Structure") (User :type "Actor Object Reference"))
  ;[1 1 1] Gives the player one berry and starts a cooldown
  (set `self.IsCoolingDown` true)
  (bind _returnvalue (`KismetSystemLibrary.K2_SetTimerDelegate` (delegate `OnCooldownEnded`) (`self.CoolDownTime`)))
  (set `self.PickupCooldown` _returnvalue)
  (bind _asbp_interaction_character (cast `/Game/InteractionExamples/Character/BP_InteractionCharacter` User))
  (`/Game/InteractionExamples/Character/BP_InteractionCharacter.AddBerry` _asbp_interaction_character))

(event `OnCooldownEnded`
  ;[1 1 1] Gives the player one berry and starts a cooldown
  (set `self.IsCoolingDown` false))

(fn `GetActionPickName`
  (params (Handle :type "InterativeActionHandle Structure") (User :type "Actor Object Reference"))
  (returns (Name :type Text))
  (bind _returnvalue (`KismetSystemLibrary.K2_GetTimerRemainingTimeHandle` (`self.PickupCooldown`)))
  (if (> _returnvalue 0.0)
    (return (`KismetTextLibrary.Conv_StringToText` (`KismetStringLibrary.BuildString_Int` "Pick Berry" ": available in " (`KismetMathLibrary.FCeil` _returnvalue) "s")))
    (else
      (return "Pick Berry"))))

(fn `GetActionPickVisibility`
  (params (Handle :type "InterativeActionHandle Structure") (User :type "Actor Object Reference"))
  (returns (Visibility :type "EInteractionVisibility Enum"))
  (if (`self.IsCoolingDown`)
    (return "DISABLED")
    (else
      (return "ENABLED"))))

(fn `UserConstructionScript`)