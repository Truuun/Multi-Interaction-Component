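; BP_InteractionHUD is a HUD that manages the crosshair and interaction menu widgets for the interaction example.
; On BeginPlay it creates both widgets for the owning player and adds them to the viewport, with the menu hidden.
; Opening the menu swaps out the crosshair and passes the component to it; closing restores game-only input, hides the cursor and shows the crosshair.
; SetCurrentInteraction forwards the current target to the crosshair widget.
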(event `self.ReceiveBeginPlay`
  ;[1 1 1] Create the HUD widgets
  (`|ExecutionSequence`
    (:`then_0`
      (bind _returnvalue (`|CreateWidget` "/Game/InteractionExamples/UI/WBP_Interact.WBP_Interact_C" (`self.PlayerOwner`)))
      (bind _output_get (set `self.InteractWidget` _returnvalue))
      (`UserWidget.AddToViewport` _output_get 0)
      (`Widget.SetVisibility` (`self.InteractWidget`) "Hidden"))
    (:`then_1`
      (bind _returnvalue_2 (`|CreateWidget` "/Game/InteractionExamples/UI/WBP_Crosshair.WBP_Crosshair_C" (`self.PlayerOwner`)))
      (bind _output_get_2 (set `self.CrosshairWidget` _returnvalue_2))
      (`UserWidget.AddToViewport` _output_get_2 0))))

(fn `CloseInteractMenu`
  (bind _playerowner (`self.PlayerOwner`))
  ;[1 1 1] Show crosshair and hide menu
  (`WidgetBlueprintLibrary.SetInputMode_GameOnly` _playerowner)
  (set `PlayerController.bShowMouseCursor` false _playerowner)
  (`/Game/InteractionExamples/UI/WBP_Interact.Close` (`self.InteractWidget`))
  (`Widget.SetVisibility` (`self.CrosshairWidget`) "Visible"))

(fn `OpenInteractMenu`
  (params (Component :type "MultiInteractionComponent Object Reference"))
  (bind _interactwidget (`self.InteractWidget`))
  ;[1 1 1] Hide the crosshair and show the interaction menu
  (`Widget.SetVisibility` (`self.CrosshairWidget`) "Hidden")
  (`Widget.SetVisibility` _interactwidget "Visible")
  (`/Game/InteractionExamples/UI/WBP_Interact.OnOpen` _interactwidget Component))

(fn `SetCurrentInteraction`
  (params (NewParam :type "MultiInteractionComponent Object Reference"))
  (`/Game/InteractionExamples/UI/WBP_Crosshair.SetObject` (`self.CrosshairWidget`) NewParam))

(fn `UserConstructionScript`)